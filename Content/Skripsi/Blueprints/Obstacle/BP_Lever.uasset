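; BP_Lever is a lever obstacle with an open or closed state, shown by the tilt of its handle.
; SetOpen either plays the LeverAnimation timeline forward or backward to swing the handle's roll, or snaps it straight to the end angle.
; Only non-animated calls record the state as OpenOri, which Reset reapplies without animation to restore the lever's original position.
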(event `SetOpen`
  (params (open :type Boolean) (animate :type Boolean))
  (set `self.open` open)
  (set `self.animate` animate)
  (if (`self.animate`)
    (if (`self.open`)
      (bind (_direction _alpha) (`Timeline|LeverAnimation` :!via `PlayFromStart` :!label _label)
        (:`Update`
          (`SceneComponent.K2_SetRelativeRotation` (`self.Lever Handle`) (`KismetMathLibrary.MakeRotator` (`KismetMathLibrary.Lerp` 45.0 -45.0 _alpha)) false false)))
      (else
        (goto _label :!via `ReverseFromEnd`)))
    (else
      (set `self.openOri` (`self.open`))
      (if (`self.open`)
        (`SceneComponent.K2_SetRelativeRotation` (`self.Lever Handle`) (struct :`Roll` -45.0) false false)
        (else
          (`SceneComponent.K2_SetRelativeRotation` (`self.Lever Handle`) (struct :`Roll` 45.0) false false))))))

(fn `Reset`
  (`self.SetOpen` (`self.openOri`)))

(fn `UserConstructionScript`
  (`parent.UserConstructionScript`))