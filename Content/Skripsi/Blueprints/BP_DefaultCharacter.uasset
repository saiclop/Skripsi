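; BP_DefaultCharacter is a character Blueprint that turns keyboard presses into player movement commands.
; Number keys 1–3 call turn right, turn left and move forward, while WASD and F call PlayerMove with an enum value, and Z calls a position reset.
; The graph only relays these calls, which appear to be event dispatchers, and contains no movement logic; BeginPlay and the construction script are empty.
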(event `self.ReceiveBeginPlay`)

(event `Key|One`
  (params (Key :type "Key Structure"))
  (:`Pressed`
    (`self.PlayerTurnRight`)))

(event `Key|Two`
  (params (Key :type "Key Structure"))
  (:`Pressed`
    (`self.PlayerTurnLeft`)))

(event `Key|Three`
  (params (Key :type "Key Structure"))
  (:`Pressed`
    (`self.PlayerMoveForward`)))

(event `Key|A`
  (params (Key :type "Key Structure"))
  (:`Pressed`
    (`self.PlayerMove` "NewEnumerator3")))

(event `Key|S`
  (params (Key :type "Key Structure"))
  (:`Pressed`
    (`self.PlayerMove` "NewEnumerator2")))

(event `Key|D`
  (params (Key :type "Key Structure"))
  (:`Pressed`
    (`self.PlayerMove` "NewEnumerator1")))

(event `Key|W`
  (params (Key :type "Key Structure"))
  (:`Pressed`
    (`self.PlayerMove` "NewEnumerator0")))

(event `Key|F`
  (params (Key :type "Key Structure"))
  (:`Pressed`
    (`self.PlayerMove` "NewEnumerator4")))

(event `Key|Z`
  (params (Key :type "Key Structure"))
  (:`Pressed`
    (`self.ResetPosition`)))

(fn `UserConstructionScript`)